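; BP_EnemyTest is a test enemy that loses health when player 0 damages it.
; Its AnyDamage event accepts only damage instigated by that player's controller, and ignores it when the TopDownCharacter's Alliance equals 1.
; Health is checked before damage is subtracted, so the actor is destroyed on the next accepted hit after CurrentHealth reaches zero or below.
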(event `self.ReceiveAnyDamage`
  (params (Damage :type "Float (single-precision)") (DamageType :type "DamageType Object Reference") (InstigatedBy :type "Controller Object Reference") (DamageCauser :type "Actor Object Reference"))
  (if (== InstigatedBy (`GameplayStatics.GetPlayerController` 0))
    (bind _astop_down_character (cast `/Game/TopDownBP/Blueprints/TopDownCharacter` (`GameplayStatics.GetPlayerCharacter` 0)))
    (if (== (`/Game/TopDownBP/Blueprints/TopDownCharacter.Alliance` _astop_down_character) 1)
      _
      (elif (<= (`self.CurrentHealth`) 0.0)
        (set `self.CurrentHealth` 0.0)
        (`self.K2_DestroyActor`)
        (else
          (set `self.CurrentHealth` (- (`self.CurrentHealth`) Damage)))))))

(fn `UserConstructionScript`)