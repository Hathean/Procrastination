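; BP_BulletTest is a test bullet actor that damages what it overlaps and destroys itself after five seconds.
; On overlap, it looks the other actor up among all actors of its class, applies BulletDamage crediting player controller 0, then destroys itself.
; The class-wide searches effectively resolve back to the overlapped actor.
; The Hit event only gathers actors of the hit class without using them, and no movement logic appears in the graphs.
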(event `self.ReceiveBeginPlay`
  (`KismetSystemLibrary.Delay` 5.0)
  (`self.K2_DestroyActor`))

(event `self.ReceiveActorBeginOverlap`
  (params (OtherActor :type "Actor Object Reference"))
  (bind _returnvalue (`GameplayStatics.GetObjectClass` OtherActor))
  (bind _outactors (`GameplayStatics.GetAllActorsOfClass` _returnvalue))
  (bind _returnvalue_2 (`KismetArrayLibrary.Array_Find` _outactors OtherActor))
  (if (== OtherActor (`|GetArrayItem` _outactors _returnvalue_2))
    (bind _outactors_2 (`GameplayStatics.GetAllActorsOfClass` _returnvalue))
    (`GameplayStatics.ApplyDamage` (`|GetArrayItem` _outactors_2 _returnvalue_2) (`self.BulletDamage`) (`GameplayStatics.GetPlayerController` 0) self "/Script/Engine.DamageType"))
  (`self.K2_DestroyActor`))

(event `self.ReceiveHit`
  (params (MyComp :type "PrimitiveComponent Object Reference") (Other :type "Actor Object Reference") (OtherComp :type "PrimitiveComponent Object Reference") (bSelfMoved :type Boolean) (HitLocation :type "Vector Structure") (HitNormal :type "Vector Structure") (NormalImpulse :type "Vector Structure") (Hit :type "HitResult Structure (by ref)"))
  (bind _outactors (`GameplayStatics.GetAllActorsOfClass` (`GameplayStatics.GetObjectClass` (`.HitActor` (`GameplayStatics.BreakHitResult` Hit))))))

(fn `UserConstructionScript`)